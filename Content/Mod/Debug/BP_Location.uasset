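; BP_Location is a debug widget component that shows its owner's position and velocity as screen-space text.
; Each tick it derives velocity from the change in the owner's Y/Z location over delta time, treating that plane as 2D.
; The DMOwner's Enabled flag controls visibility, while AnceyEnabled also keeps the values updating.
; The text is blanked when the owner or its Spine renderer is hidden or its red channel is near zero.
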(event `self.ReceiveBeginPlay`
  (bind _returnvalue (`|CreateWidget` "/Game/Mod/Debug/WBP_Text.WBP_Text_C"))
  (set `self.text` _returnvalue)
  (`self.SetWidget` _returnvalue)
  (set `self.renderer` (`Actor.GetComponentByClass` (`self.GetOwner`) "/Script/SpinePlugin.SpineSkeletonRendererComponent"))
  (`self.SetWidgetSpace` "Screen")
  (bind _aszenith_companion_character (cast `ZenithCompanionCharacter` (`self.GetOwner`)))
  (set `self.As Zenith Companion Character` _aszenith_companion_character))

(event `self.ReceiveTick`
  (params (DeltaSeconds :type "Float (single-precision)"))
  (set `self.deltaT` DeltaSeconds)
  (bind _dm_owner (`self.DM_Owner`)
    (:`then`
      (`|ExecutionSequence`
        (:`then_0`
          (bind _enabled (`/Game/Mod/Debug/DebugModules/DM_ShowLocation.enabled` _dm_owner))
          (`self.SetHiddenInGame` (not _enabled))
          (if (or _enabled (`/Game/Mod/Debug/DebugModules/DM_ShowLocation.AnceyEnabled` _dm_owner))
            (`self.SetVar`)))
        (:`then_1`
          (if _enabled
            (`self.SetLText`)))))
    (:`else`
      (`self.SetHiddenInGame` true)
      (`self.SetVar`))))

(event `SetVar`
  (bind _lx (`self.lx`))
  (bind _ly (`self.ly`))
  (bind _deltat (`self.deltaT`))
  (bind (_x _y) (`KismetMathLibrary.BreakVector2D` (`self.LastLocation`)))
  (if (> (`self.deltaT`) 0.001)
    (set `self.lx` (.y (`Actor.K2_GetActorLocation` (`self.GetOwner`))))
    (set `self.ly` (.z (`Actor.K2_GetActorLocation` (`self.GetOwner`))))
    (set `self.vx` (/ (- _lx _x) _deltat))
    (set `self.vy` (/ (- _ly _y) _deltat))
    (set `self.LastLocation` (`KismetMathLibrary.MakeVector2D` _lx _ly))))

(event `SetLText`
  (bind _renderer (`self.renderer`))
  (bind _color_r (break `LinearColor` (`SpineSkeletonRendererComponent.Color` _renderer)))
  (`/Game/Mod/Debug/WBP_Text.SetText` (`self.text`) (select `bool` (and (not (`SceneComponent.bHiddenInGame` _renderer)) (not (`Actor.bHidden` (`self.GetOwner`))) (`SceneComponent.bVisible` _renderer) (> _color_r 0.01)) :`true` (`|FormatText` " \n({x},{y}) v:({z},{w})" (`KismetTextLibrary.Conv_DoubleToText` (`self.lx`) "HalfToEven" false true 1 324 3) (`KismetTextLibrary.Conv_DoubleToText` (`self.ly`) "HalfToEven" false true 1 324 3) (`KismetTextLibrary.Conv_DoubleToText` (`self.vx`) "HalfToEven" false true 1 324 3) (`KismetTextLibrary.Conv_DoubleToText` (`self.vy`) "HalfToEven" false true 1 324 3)))))