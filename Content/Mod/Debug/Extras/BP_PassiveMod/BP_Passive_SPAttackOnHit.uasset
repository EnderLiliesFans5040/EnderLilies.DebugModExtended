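; BP_Passive_SPAttackOnHit is a debug passive mod that force-kills the target reported by the player's got-parried event, despite its SP-attack-on-hit name.
; Applying it to a pawn casts that pawn to ZenithCharacter and binds to its got-parried delegate, with a stored flag and player check guarding against rebinding.
; When the delegate fires, the target's DeathComponent forces death if the target is a ZenithCharacter.
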(event `Bind`
  (params (Player :type "Pawn Object Reference"))
  (bind _player (`self.player`)
    (:`then`
      (if (not (and (`self.Binded`) (== _player Player)))
        (bind _aszenith_character (cast `ZenithCharacter` Player :!label _label))
        (bind _output_get (set `self.player` _aszenith_character))
        (add `ZenithCharacter.OnGotParriedDelegate` _output_get (delegate `OnGotParriedDelegate_Event`))
        (set `self.Binded` true)))
    (:`else`
      (goto _label))))

(event `OnGotParriedDelegate_Event`
  (params (Ability :type "Ability Object Reference") (Target :type "Actor Object Reference"))
  (bind _aszenith_character (cast `ZenithCharacter` Target))
  (`DeathComponent.ForceDeath` (`ZenithCharacter.DeathComponent` _aszenith_character)))

(event `self.OnApplyToPawn`
  (params (Pawn :type "Pawn Object Reference") (Controller :type "Controller Object Reference"))
  (`self.Bind` Pawn))