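; BP_OverheadText is a debug widget component that shows the owning actor's current Spine animation name as screen-space text.
; On BeginPlay it creates a WBP_Text widget, caches the owner's Spine animation and renderer components, and casts the owner to ZenithCompanionCharacter.
; Each tick, DMOwner's Enabled flag controls visibility, and the text blanks when the owner or renderer is hidden or the renderer's red channel is near zero.
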(event `self.ReceiveBeginPlay`
  (bind _returnvalue (`self.GetOwner`))
  (bind _returnvalue_2 (`|CreateWidget` "/Game/Mod/Debug/WBP_Text.WBP_Text_C"))
  (set `self.text` _returnvalue_2)
  (`self.SetWidget` _returnvalue_2)
  (set `self.spine` (`Actor.GetComponentByClass` _returnvalue "/Script/Zenith.SpineAnimationComponent"))
  (set `self.renderer` (`Actor.GetComponentByClass` _returnvalue "/Script/SpinePlugin.SpineSkeletonRendererComponent"))
  (`self.SetWidgetSpace` "Screen")
  (bind _aszenith_companion_character (cast `ZenithCompanionCharacter` (`self.GetOwner`)))
  (set `self.As Zenith Companion Character` _aszenith_companion_character))

(event `self.ReceiveTick`
  (params (DeltaSeconds :type "Float (single-precision)"))
  (bind _renderer (`self.renderer`))
  (bind _color_r (break `LinearColor` (`SpineSkeletonRendererComponent.Color` _renderer)))
  (bind _dm_owner (`self.DM_Owner`)
    (:`then`
      (bind _enabled (`/Game/Mod/Debug/DebugModules/DM_ShowAnimations.enabled` _dm_owner))
      (`self.SetHiddenInGame` (not _enabled))
      (if _enabled
        (bind _spine (`self.spine`)
          (:`then`
            (`/Game/Mod/Debug/WBP_Text.SetText` (`self.text`) (select `bool` (and (not (`SceneComponent.bHiddenInGame` _renderer)) (not (`Actor.bHidden` (`self.GetOwner`))) (`SceneComponent.bVisible` _renderer) (> _color_r 0.01)) :`true` (`KismetTextLibrary.Conv_StringToText` (`KismetStringLibrary.Concat_StrStr` (`SpineAnimationComponent.GetCurrentAnimationName` _spine) " \n")))))
          (:`else`))))
    (:`else`)))