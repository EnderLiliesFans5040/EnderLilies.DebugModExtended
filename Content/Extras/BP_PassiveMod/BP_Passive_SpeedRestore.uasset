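; Passive mod that refunds command use counts and cooldowns when the player damages a moving enemy.
; Applying it binds the player's damage delegate; removing it only disables restoring.
; Each hit reads the enemy's BP_Location XY speed, converts it to a capped ratio, and restores cooldown at double that ratio.
; Toggling also sets AnceyEnabled through the player's BP_Location, or adds that component if missing.
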(event `Bind`
  (params (player :type "Pawn Object Reference (by ref)"))
  (bind _player (`self.player`)
    (:`then`
      (if (not (and (`self.Binded`) (== _player player)))
        (bind _aszenith_character (cast `ZenithCharacter` player :!label _label))
        (bind _output_get (set `self.player` _aszenith_character))
        (add `ZenithCharacter.OnDamagedEnemyDelegate` _output_get (delegate `OnDamagedEnemyDelegate_Event`))
        (set `self.Binded` true)))
    (:`else`
      (goto _label))))

(event `OnDamagedEnemyDelegate_Event`
  (params (DamagedEnemy :type "Actor Object Reference") (DamageDone :type Integer))
  (bind _output_get (set `self.enemyBP` (`Actor.GetComponentByClass` DamagedEnemy "/Game/Mod/Debug/BP_Location.BP_Location_C")))
  (`/Engine/EditorBlueprintResources/StandardMacros.IsValid` _output_get
    (:`Is Valid`
      (bind _output_get_2 (set `self.v` (`self.GetLengthByXY` (`/Game/Mod/Debug/BP_Location.vx` _output_get) (`/Game/Mod/Debug/BP_Location.vy` _output_get))))
      (if (not (`KismetMathLibrary.NearlyEqual_FloatFloat` 0.0 _output_get_2))
        (`self.RestoreByRatio` (`KismetMathLibrary.FMin` 0.05 (+ (* _output_get_2 0.0001) 0.02)))))))

(event `self.OnApplyToPawn`
  (params (Pawn :type "Pawn Object Reference") (Controller :type "Controller Object Reference"))
  (`self.Bind` Pawn)
  (`self.SetAnceyEnabled` true))

(event `self.OnRemoveFromPawn`
  (params (Pawn :type "Pawn Object Reference") (Controller :type "Controller Object Reference"))
  (`self.SetAnceyEnabled` false))

(event `self.OnEquipPassive`
  (params (Controller :type "Controller Object Reference")))

(event `self.OnUnequipPassive`
  (params (Controller :type "Controller Object Reference")))

(event `RestoreByRatio`
  (params (ratio :type "Float (double-precision)"))
  (bind _commandqueuecomponent (`ZenithCharacter.CommandQueueComponent` (`self.player`)))
  (if (`self.Enabled`)
    (`CommandQueueComponent.RestoreUseCountByRatio` _commandqueuecomponent ratio)
    (`CommandQueueComponent.RestoreCooldownByRatio` _commandqueuecomponent (* 2 ratio))))

(event `SetAnceyEnabled`
  (params (Ancey :type Boolean))
  (bind _returnvalue (`Actor.GetComponentByClass` (`self.player`) "/Game/Mod/Debug/BP_Location.BP_Location_C"))
  (bind _output_get (set `self.Enabled` Ancey))
  (`/Engine/EditorBlueprintResources/StandardMacros.IsValid` _returnvalue
    (:`Is Valid`
      (set `/Game/Mod/Debug/DebugModules/DM_ShowLocation.AnceyEnabled` _output_get (`/Game/Mod/Debug/BP_Location.DM_Owner` _returnvalue)))
    (:`Is Not Valid`
      (`|AddComponentByClass` (`self.player`) "/Game/Mod/Debug/BP_Location.BP_Location_C" false (`KismetMathLibrary.MakeTransform` (0.0 0.0 0.0)) null))))