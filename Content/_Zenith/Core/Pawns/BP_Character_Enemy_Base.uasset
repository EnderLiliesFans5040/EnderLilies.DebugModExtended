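; BP_Character_Enemy_Base is the base Blueprint for enemy characters, mostly a skeleton of hooks.
; Begin play, landing, movement-mode changes, respawn, construction and sort priority defer to the parent class, while overlap and Tick are disabled.
; Target, pause, contact damage and meat-action functions are stubs returning empty or default values.
; A FadeOut timeline and the target-change and swimming events exist with no logic attached.
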(event `self.ReceiveBeginPlay`
  (`parent.ReceiveBeginPlay`))

(event `FadeOut__FinishedFunc`)

(event `FadeOut__UpdateFunc`)

(event `self.OnLanded`
  (params (Hit :type "HitResult Structure (by ref)"))
  (`parent.OnLanded` Hit))

(event `OnChangeTarget`
  (params (NewTarget :type "Actor Object Reference")))

(event `self.K2_OnMovementModeChanged`
  (params (PrevMovementMode :type "EMovementMode Enum" :default "MOVE_None") (NewMovementMode :type "EMovementMode Enum" :default "MOVE_None") (PrevCustomMode :type Byte) (NewCustomMode :type Byte))
  (`parent.K2_OnMovementModeChanged` PrevMovementMode NewMovementMode PrevCustomMode NewCustomMode))

(event `OnMovementModeChanged_ToSwimming`)

(event `self.OnRespawn`
  (`parent.OnRespawn`))

(fn `ComputeSortPriority`
  (returns (SortPriority :type Integer))
  (bind _sortpriority (`parent.ComputeSortPriority`))
  (return _sortpriority))

(fn `GetContactDamage`
  (returns (ContactDamage :type Integer))
  (return 0))

(fn `GetCurrentTarget`
  (returns (CurrentTarget :type "Actor Object Reference"))
  (return null))

(fn `IsPaused`
  (returns (Paused :type Boolean))
  (return false))

(fn `PlayMeatAction`)

(fn `SetPaused`
  (params (Paused :type Boolean)))

(fn `StopMeatAction`)

(fn `UserConstructionScript`
  (`parent.UserConstructionScript`))