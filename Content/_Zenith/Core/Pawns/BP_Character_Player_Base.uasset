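; BP_Character_Player_Base is a player character base Blueprint that mostly forwards to its parent class.
; BeginPlay, submersion, movement-mode change and just-guard events call their parent versions, as does the construction script.
; Functions for aptitude unlocks, auto-dive, contact damage and spine data are stubs that are empty or return false or zero.
; The DamageColorCurve timeline callbacks are empty, and Tick and overlap events are disabled.
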(event `self.ReceiveBeginPlay`
  (`parent.ReceiveBeginPlay`))

(event `DamageColorCurve__FinishedFunc`)

(event `DamageColorCurve__UpdateFunc`)

(event `OnFinish_9EDCDC9446133E62BE79C0B3D03533F1`)

(event `self.OnSubmerged`
  (`parent.OnSubmerged`))

(event `self.K2_OnMovementModeChanged`
  (params (PrevMovementMode :type "EMovementMode Enum" :default "MOVE_None") (NewMovementMode :type "EMovementMode Enum" :default "MOVE_None") (PrevCustomMode :type Byte) (NewCustomMode :type Byte))
  (`parent.K2_OnMovementModeChanged` PrevMovementMode NewMovementMode PrevCustomMode NewCustomMode))

(event `self.OnJustGuard`
  (params (Ability :type "Ability Object Reference") (Invoker :type "Actor Object Reference") (bWillForwardEventToAttacker :type Boolean))
  (`parent.OnJustGuard` Ability Invoker bWillForwardEventToAttacker))

(fn `FindSpineDataForLevel`
  (returns (Result :type Boolean) (SpindDataGroup :type "/Game/_Zenith/Gameplay/Structures/FSpineDataGroup Structure"))
  (return false))

(fn `GetContactDamage`
  (params (EnemyCharacter :type "/Game/_Zenith/Core/Pawns/BP_Character_Enemy_Base Object Reference"))
  (returns (ContactDamage :type Integer))
  (return 0))

(fn `IsPlayerAptitudeUnlocked`
  (params (Aptitude :type "EAptitudeType Enum" :default "None"))
  (returns (ReturnValue :type Boolean))
  (return false))

(fn `RefreshSpineData`
  (returns (Changed :type Boolean))
  (return false))

(fn `SetSpineData`
  (params (FSpineDataGroup :type "/Game/_Zenith/Gameplay/Structures/FSpineDataGroup Structure (by ref)")))

(fn `ShouldTriggerAutoDive`
  (returns (ReturnValue :type Boolean))
  (return false))

(fn `UserConstructionScript`
  (`parent.UserConstructionScript`))