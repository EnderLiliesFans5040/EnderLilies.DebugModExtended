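; Base character Blueprint for boss pawns, with almost no logic of its own.
; BeginPlay, possession and construction defer to the parent class, while overlap and Tick are disabled.
; Death-process, death-animation, death-event, timeline and finish callbacks are empty, as is the death-event blackboard setup.
; The conditioned conversation data query always returns false.
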(event `self.ReceiveBeginPlay`
  (`parent.ReceiveBeginPlay`))

(event `Timeline_0__FinishedFunc`)

(event `Timeline_0__UpdateFunc`)

(event `OnFinish_94D3316D428E3071DF0952A4CFD5AC4B`)

(event `OnDeathEventFinished`)

(event `OnDeathProcessStart`)

(event `OnDeathAnimationComplete`)

(event `self.ReceivePossessed`
  (params (NewController :type "Controller Object Reference"))
  (`parent.ReceivePossessed` NewController))

(fn `GetConditionedConversationData`
  (returns (Result :type Boolean) (Conversation :type "ConversationData Structure"))
  (return false))

(fn `SetupDeathEventBlackboard`
  (params (EventPlayer :type "EventPlayer Object Reference")))

(fn `UserConstructionScript`
  (`parent.UserConstructionScript`))