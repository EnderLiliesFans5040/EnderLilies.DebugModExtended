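; BP_Character_Base is a base character Blueprint under the project's core pawns, acting mostly as a skeleton.
; Its just-guard, landing, unpossess and movement-mode events only forward to the parent implementations, while BeginPlay, overlap and Tick are disabled.
; SimulateLanding is an empty stub, and CanPlayLandingEvents and CanBePossessed both return false as defaults.
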(event `self.OnJustGuard`
  (params (Ability :type "Ability Object Reference") (Invoker :type "Actor Object Reference") (bWillForwardEventToAttacker :type Boolean))
  (`parent.OnJustGuard` Ability Invoker bWillForwardEventToAttacker))

(event `self.OnLanded`
  (params (Hit :type "HitResult Structure (by ref)"))
  (`parent.OnLanded` Hit))

(event `self.ReceiveUnpossessed`
  (params (OldController :type "Controller Object Reference"))
  (`parent.ReceiveUnpossessed` OldController))

(event `self.K2_OnMovementModeChanged`
  (params (PrevMovementMode :type "EMovementMode Enum" :default "MOVE_None") (NewMovementMode :type "EMovementMode Enum" :default "MOVE_None") (PrevCustomMode :type Byte) (NewCustomMode :type Byte))
  (`parent.K2_OnMovementModeChanged` PrevMovementMode NewMovementMode PrevCustomMode NewCustomMode))

(event `self.OnGotJustGuarded`
  (params (Ability :type "Ability Object Reference") (Target :type "Actor Object Reference"))
  (`parent.OnGotJustGuarded` Ability Target))

(fn `CanBePossessed`
  (returns (CanBePossessed :type Boolean))
  (return false))

(fn `CanPlayLandingEvents`
  (returns (ReturnValue :type Boolean))
  (return false))

(fn `SimulateLanding`
  (params (Size :type "Float (double-precision)") (Strength :type "Float (double-precision)")))

(fn `UserConstructionScript`)