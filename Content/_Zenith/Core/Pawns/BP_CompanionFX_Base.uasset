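; Base companion FX Blueprint that serves as an overridable shell, with almost no logic of its own.
; Lifecycle, activation, spine show/hide, visibility, translucency and spirit-data events mostly just forward to the parent class.
; FadeIn/FadeOut timeline handlers and hooks for teleport, world-space UI, dissolve and idle animation overrides are empty.
; Getters for UI offset, FX color and idle animation name return neutral defaults.
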(event `self.ReceiveBeginPlay`
  (`parent.ReceiveBeginPlay`))

(event `self.ReceiveTick`
  (params (DeltaSeconds :type "Float (single-precision)"))
  (`parent.ReceiveTick` DeltaSeconds))

(event `FadeIn__FinishedFunc`)

(event `FadeIn__UpdateFunc`)

(event `FadeOut__FinishedFunc`)

(event `FadeOut__UpdateFunc`)

(event `self.OnShowSpine`
  (`parent.OnShowSpine`))

(event `self.OnHideSpine`
  (`parent.OnHideSpine`))

(event `self.OnSetMeshComponentsHiddenInGame`
  (params (bHiddenInGame :type Boolean))
  (`parent.OnSetMeshComponentsHiddenInGame` bHiddenInGame))

(event `SetPoseFadePlaneAlpha`
  (params (Alpha :type "Float (double-precision)")))

(event `self.OnActivate`
  (`parent.OnActivate`))

(event `self.OnDeactivate`
  (`parent.OnDeactivate`))

(event `self.ReceiveEndPlay`
  (params (EndPlayReason :type "EEndPlayReason Enum" :default "Destroyed"))
  (`parent.ReceiveEndPlay` EndPlayReason))

(event `self.ReceiveDestroyed`
  (`parent.ReceiveDestroyed`))

(event `self.OnSetTranslucencyPriority`
  (params (Priority :type Integer))
  (`parent.OnSetTranslucencyPriority` Priority))

(event `self.OnEventStop`
  (`parent.OnEventStop`))

(event `OnAssociatedCommandStart`)

(event `self.OnSetAssociatedSpiritData`
  (`parent.OnSetAssociatedSpiritData`))

(fn `ClearIdleAnimationOverride`)

(fn `GetDesiredFXColor`
  (returns (DesiredColor :type "LinearColor Structure"))
  (return))

(fn `GetDesiredUIOffset`
  (returns (ReturnValue :type "Vector Structure"))
  (return (0.0 0.0 0.0)))

(fn `GetIdleAnimationName`
  (returns (IdleAnimationName :type String))
  (return ""))

(fn `Set FXVisibility`
  (params (Visible :type Boolean)))

(fn `SetDissolveValue`
  (params (DissolveValue :type "Float (double-precision)")))

(fn `SetIdleAnimationOverride`
  (params (IdleAnimationOverrideName :type String)))

(fn `TeleportToAssociatedLocation`)

(fn `TriggerWorldSpaceUI`)

(fn `UserConstructionScript`)