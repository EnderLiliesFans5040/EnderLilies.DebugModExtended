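; BP_Passive_StaminaUp is a passive that restores command use counts and cooldowns when the player damages enemies.
; Applying it binds to the ZenithCharacter's damaged-enemy delegate; removing it runs the same bind and also leaves it enabled.
; Each hit derives a ratio from the damaged enemy's speed, ignoring damage dealt, and feeds it to the player's CommandQueueComponent, doubled for cooldowns.
; Equip and unequip events do nothing.
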(event `Bind`
  (params (player :type "Pawn Object Reference (by ref)"))
  (bind _player (`self.player`)
    (:`then`
      (if (not (and (`self.Binded`) (== _player player)))
        (bind _aszenith_character (cast `ZenithCharacter` player :!label _label))
        (bind _output_get (set `self.player` _aszenith_character))
        (add `ZenithCharacter.OnDamagedEnemyDelegate` _output_get (delegate `OnDamagedEnemyDelegate_Event`))
        (set `self.Binded` true)))
    (:`else`
      (goto _label))))

(event `OnDamagedEnemyDelegate_Event`
  (params (DamagedEnemy :type "Actor Object Reference") (DamageDone :type Integer))
  (`self.RestoreByRatio` (* 0.01 (`KismetMathLibrary.VSize` (`Actor.GetVelocity` DamagedEnemy)))))

(event `self.OnApplyToPawn`
  (params (Pawn :type "Pawn Object Reference") (Controller :type "Controller Object Reference"))
  (`self.Bind` Pawn)
  (set `self.Enabled` true))

(event `self.OnRemoveFromPawn`
  (params (Pawn :type "Pawn Object Reference") (Controller :type "Controller Object Reference"))
  (`self.Bind` Pawn)
  (set `self.Enabled` true))

(event `self.OnEquipPassive`
  (params (Controller :type "Controller Object Reference")))

(event `self.OnUnequipPassive`
  (params (Controller :type "Controller Object Reference")))

(event `RestoreByRatio`
  (params (ratio :type "Float (double-precision)"))
  (bind _commandqueuecomponent (`ZenithCharacter.CommandQueueComponent` (`self.player`)))
  (if (`self.Enabled`)
    (`CommandQueueComponent.RestoreUseCountByRatio` _commandqueuecomponent ratio)
    (`CommandQueueComponent.RestoreCooldownByRatio` _commandqueuecomponent (* 2 ratio))))