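; Water physics volume Blueprint that declares hooks for actor entry and exit, splashes, audio and post-process blending.
; Function names outline size-based enter/exit events, player and ability hitbox checks, reverb and snapshot triggers, and render-target wave helpers for surface location and FX.
; All of these are empty stubs or return defaults.
; Only BeginPlay and Tick do anything, forwarding to the parent class.
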(event `self.ReceiveBeginPlay`
  (`parent.ReceiveBeginPlay`))

(event `self.ReceiveTick`
  (params (DeltaSeconds :type "Float (single-precision)"))
  (`parent.ReceiveTick` DeltaSeconds))

(event `PostProcessBlend__FinishedFunc`)

(event `PostProcessBlend__UpdateFunc`)

(event `DisableReverb`)

(event `EnableReverb`)

(event `OnActorEnter_Large`
  (params (Actor :type "Actor Object Reference")))

(event `OnActorExit_Large`
  (params (Actor :type "Actor Object Reference")))

(event `OnActorEnter_Medium`
  (params (Actor :type "Actor Object Reference")))

(event `OnActorExit_Medium`
  (params (Actor :type "Actor Object Reference")))

(event `Splash`
  (params (InVec :type "Vector Structure") (Size :type "Float (double-precision)") (Strength :type "Float (double-precision)")))

(event `BlendInPostProcess`)

(event `BlendOutPostProcess`)

(fn `ApplyInteractingActorSplashes`)

(fn `CheckAbilityHitboxEnter`
  (params (Actor :type "Actor Object Reference")))

(fn `CheckPlayerEnter`
  (params (Object :type "Object Object Reference")))

(fn `CheckPlayerExit`
  (params (Actor :type "Object Object Reference")))

(fn `GetActorLocationOnWave`
  (params (Target :type "Actor Object Reference"))
  (returns (Location :type "Vector Structure"))
  (return (0.0 0.0 0.0)))

(fn `GetAudioSnapshotTag`
  (returns (ReturnValue :type Name))
  (return "None"))

(fn `GetHeightRT`
  (params (CurrentHeightIndex :type Integer) (NumFrameOld :type Integer))
  (returns (Output :type "TextureRenderTarget2D Object Reference"))
  (return null))

(fn `GetLocationOnSurface`
  (params (Actor :type "Actor Object Reference"))
  (returns (BoxSide :type "EBoxSide Enum") (ReturnValue :type "Vector Structure"))
  (return "None" (0.0 0.0 0.0)))

(fn `PlayFXAtActorLocation`
  (params (Actor :type "Actor Object Reference") (bLargeFX :type Boolean)))

(fn `SetupAudioSnapshotTrigger`)

(fn `UserConstructionScript`)

(fn `WorldSpaceToUVSpace`
  (params (InVec :type "Vector Structure"))
  (returns (UV :type "LinearColor Structure"))
  (return))