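; Character Blueprint for Lily (p0000), a child class that adds no logic of its own in these graphs.
; BeginPlay, crouch start and end, construction, Spine data setup and camera focus target lookup all defer to the parent implementation.
; Tick and actor overlap events are disabled placeholder nodes.
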(event `self.ReceiveBeginPlay`
  (`parent.ReceiveBeginPlay`))

(event `self.K2_OnStartCrouch`
  (params (HalfHeightAdjust :type "Float (single-precision)") (ScaledHalfHeightAdjust :type "Float (single-precision)"))
  (`parent.K2_OnStartCrouch` HalfHeightAdjust ScaledHalfHeightAdjust))

(event `self.K2_OnEndCrouch`
  (params (HalfHeightAdjust :type "Float (single-precision)") (ScaledHalfHeightAdjust :type "Float (single-precision)"))
  (`parent.K2_OnEndCrouch` HalfHeightAdjust ScaledHalfHeightAdjust))

(fn `GetCameraFocusTarget`
  (returns (ReturnValue :type "SceneComponent Object Reference"))
  (return (`parent.GetCameraFocusTarget`)))

(fn `SetSpineData`
  (params (FSpineDataGroup :type "/Game/_Zenith/Gameplay/Structures/FSpineDataGroup Structure (by ref)"))
  (`parent.SetSpineData` FSpineDataGroup)
  (return))

(fn `UserConstructionScript`
  (`parent.UserConstructionScript`))