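; BP_e2161_Spider is a spider character Blueprint whose interface suggests a physics-driven body hanging from the ceiling on a cable.
; Events cover moving to a height from ceiling or ground, setting ceiling distance and adding force.
; Helper functions name cable and constraint setup, limit updates, height conversion and actor-to-physics syncing.
; All of these are empty or return defaults here; BeginPlay, Tick and construction only call the parent.
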(event `self.ReceiveBeginPlay`
  (`parent.ReceiveBeginPlay`))

(event `self.ReceiveTick`
  (params (DeltaSeconds :type "Float (single-precision)"))
  (`parent.ReceiveTick` DeltaSeconds))

(event `MoveToHeightFromCeiling`
  (params (Height :type "Float (double-precision)") (MoveSpeed :type "Float (double-precision)")))

(event `SetDistanceFromCeiling`
  (params (NewMaxDistance :type "Float (double-precision)")))

(event `AddForce`
  (params (Force :type "Vector Structure") (bAccelChange :type Boolean)))

(event `MoveToHeightFromGround`
  (params (Height :type "Float (double-precision)") (MoveSpeed :type "Float (double-precision)")))

(fn `ConvertToHeightFromCeiling`
  (params (HeightFromGround :type "Float (double-precision)"))
  (returns (HeightFromCeiling :type "Float (double-precision)"))
  (return 0.0))

(fn `GetCeilingLocation`
  (returns (CeilingLocation :type "Vector Structure"))
  (return (0.0 0.0 0.0)))

(fn `GetCurrentLimit`
  (returns (CurrentLimit :type "Float (double-precision)"))
  (return 0.0))

(fn `GetNewLimit`
  (params (DeltaTime :type "Float (double-precision)"))
  (returns (ReturnValue :type "Float (double-precision)"))
  (return 0.0))

(fn `InitCeilingGroundHits`
  (returns (Success :type Boolean))
  (return false))

(fn `IsAtTargetLimit`
  (returns (ReturnValue :type Boolean))
  (return false))

(fn `IsSimulatingPhysics`
  (returns (Simulating :type Boolean))
  (return false))

(fn `SetupCable`)

(fn `SetupPhysicConstraint`)

(fn `SyncActorToPhysics`)

(fn `UserConstructionScript`
  (`parent.UserConstructionScript`))